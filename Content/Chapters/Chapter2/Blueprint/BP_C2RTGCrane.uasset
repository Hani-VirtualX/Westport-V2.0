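; RTG crane actor for Chapter 2 that shows step-by-step explanation callouts and a gaze target on its ladder, walkways and floor.
; BeginPlay waits briefly, enables crane collision, caches GM_C2 and leaves Gaze set to None, though DisableGaze still resets its progress bar.
; Paired show/hide events drive VXExplain and VXGaze; the first gaze trigger calls GM_C2's Sub3212.
; Separate events swap the crane material to show or hide a hole.
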(event `self.ReceiveBeginPlay`
  (`KismetSystemLibrary.Delay` 0.2)
  (`PrimitiveComponent.SetCollisionEnabled` (`self.WP_RTGCrane_Joined`) "QueryAndPhysics")
  (bind _returnvalue (`GameplayStatics.GetActorOfClass` null))
  (set `self.Gaze` null _returnvalue)
  (bind _returnvalue_2 (`GameplayStatics.GetActorOfClass` "/Game/Chapters/Chapter2/Blueprint/GM_C2.GM_C2_C"))
  (set `self.GM_C2` _returnvalue_2))

(event `Set 1-1-1 Explain Visible`
  ;[1 0.1979 1] Explains
  (`self.Set [ Explain + ]` (`self.VX_Explain`) null (`self.1-1-1 Exp`) true 0 0 0 0 0))

(event `Set 1-1-1 Explain Hidden`
  ;[1 0.1979 1] Explains
  (`self.Set [ Explain + ]` (`self.VX_Explain`) null (`self.1-1-1 Exp`) false 0 0 0 0 0))

(event `Enable Gaze`
  ;[1 1 1] Gaze
  (`self.Set [ Gaze ]` (`self.VX_Gaze`) (`self.Cube-Walkway1`) (`self.Gaze_Label`) true 0 0 0 0))

(event `Disable Gaze`
  ;[1 1 1] Gaze
  (`self.Set [ Gaze ]` (`self.VX_Gaze`) (`self.Cube-Walkway1`) (`self.Gaze_Label`) false 0 0 0 0)
  (`self.Reset Progress Bar` (`.Gaze` (`self.Gaze`))))

(event `Set 2-1-1 Explain Visible`
  ;[1 0.1979 1] Explains
  (`self.Set [ Explain + ]` (`self.VX_Explain`) (`self.Cube-Ladder`) (`self.2-1-1 Exp`) true 0 0 0 0 0))

(event `Set 2-1-1 Explain Hidden`
  ;[1 0.1979 1] Explains
  (`self.Set [ Explain + ]` (`self.VX_Explain`) (`self.Cube-Ladder`) (`self.2-1-1 Exp`) false 0 0 0 0 0))

(event `self.VX_Gaze.Gaze Triggered`
  ;[1 1 1] Gaze
  (`/Engine/EditorBlueprintResources/StandardMacros.DoOnce` false
    (:`Completed`
      (`/Game/Chapters/Chapter2/Blueprint/GM_C2.Sub 3-2-1-2` (`self.GM_C2`)))))

(event `Set 3-1-1 Explain Visible`
  ;[1 0.1979 1] Explains
  (`self.Set [ Explain + ]` (`self.VX_Explain`) (`self.Cube-Walkway`) (`self.3-1-1 Exp`) true 0 0 0 0 0))

(event `Set 3-1-1 Explain Hidden`
  ;[1 0.1979 1] Explains
  (`self.Set [ Explain + ]` (`self.VX_Explain`) (`self.Cube-Walkway`) (`self.3-1-1 Exp`) false 0 0 0 0 0))

(event `Show Crane Hole`
  (`PrimitiveComponent.SetMaterial` (`self.WP_RTGCrane_Joined`) 0 "/Game/wesport_Stuff/Assets/RTGCrane/Materials/RTG_Bottom_Inst_Hole.RTG_Bottom_Inst_Hole"))

(event `Hide Crane Hole`
  (`PrimitiveComponent.SetMaterial` (`self.WP_RTGCrane_Joined`) 0 "/Game/wesport_Stuff/Assets/RTGCrane/Materials/RTG_Bottom_Inst.RTG_Bottom_Inst"))

(event `Set 3-1-2 Explain Visible`
  ;[1 0.1979 1] Explains
  (`self.Set [ Explain + ]` (`self.VX_Explain`) (`self.Cube-Walkway`) (`self.3-1-2 Exp`) true 0 0 0 0 0))

(event `Set 3-1-2 Explain Hidden`
  ;[1 0.1979 1] Explains
  (`self.Set [ Explain + ]` (`self.VX_Explain`) (`self.Cube-Walkway`) (`self.3-1-2 Exp`) false 0 0 0 0 0))

(event `Set 3-2-1 Explain Visible`
  ;[1 0.1979 1] Explains
  (`self.Set [ Explain + ]` (`self.VX_Explain`) (`self.Cube-Walkway`) (`self.3-2-1 Exp`) true 0 0 0 0 0))

(event `Set 3-2-1 Explain Hidden`
  ;[1 0.1979 1] Explains
  (`self.Set [ Explain + ]` (`self.VX_Explain`) (`self.Cube-Walkway`) (`self.3-2-1 Exp`) false 0 0 0 0 0))

(event `Set 3-2-2 Explain Visible`
  ;[1 0.1979 1] Explains
  (`self.Set [ Explain + ]` (`self.VX_Explain`) (`self.Cube-Walkway`) (`self.3-2-2 Exp`) true 0 0 0 0 0))

(event `Set 3-2-2 Explain Hidden`
  ;[1 0.1979 1] Explains
  (`self.Set [ Explain + ]` (`self.VX_Explain`) (`self.Cube-Walkway`) (`self.3-2-2 Exp`) false 0 0 0 0 0))

(event `Set 3-3-1 Explain Visible`
  ;[1 0.1979 1] Explains
  (`self.Set [ Explain + ]` (`self.VX_Explain`) (`self.Cube-Floor`) (`self.3-3-1 Exp`) true 0 0 0 0 0))

(event `Set 3-3-1 Explain Hidden`
  ;[1 0.1979 1] Explains
  (`self.Set [ Explain + ]` (`self.VX_Explain`) (`self.Cube-Floor`) (`self.3-3-1 Exp`) false 0 0 0 0 0))

(event `Set 3-3-5 Explain Visible`
  ;[1 0.1979 1] Explains
  (`self.Set [ Explain + ]` (`self.VX_Explain`) (`self.Cube-Floor`) (`self.3-3-5 Exp`) true 0 0 0 0 0))

(event `Set 3-3-5 Explain Hidden`
  ;[1 0.1979 1] Explains
  (`self.Set [ Explain + ]` (`self.VX_Explain`) (`self.Cube-Floor`) (`self.3-3-5 Exp`) false 0 0 0 0 0))

(event `Set 3-3-6 Explain Visible`
  ;[1 0.1979 1] Explains
  (`self.Set [ Explain + ]` (`self.VX_Explain`) (`self.Cube-Floor`) (`self.3-3-6 Exp`) true 0 0 0 0 0))

(event `Set 3-3-6 Explain Hidden`
  ;[1 0.1979 1] Explains
  (`self.Set [ Explain + ]` (`self.VX_Explain`) (`self.Cube-Floor`) (`self.3-3-6 Exp`) false 0 0 0 0 0))

(fn `UserConstructionScript`)