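; Game mode for Chapter 2 of a VR RTG crane safety training, scripting three procedures: crane explanations, hooked ladder climbing and gaze-based hazard spotting.
; BeginPlay caches level actors and the step widget; RunStepsOrder increments a counter, plays intro audio and starts the matching step.
; Numbered sub-events advance each procedure by toggling explanations, interactions and animations, reporting completed sub-procedures to the widget and ManualVR.
; Step 4 is an empty stub.
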(event `self.ReceiveBeginPlay`
  (`KismetSystemLibrary.Delay` 0.2)
  (`|ExecutionSequence`
    (:`then_0`
      (bind _gameinstance (`/Game/AFCore/Libraries/FLib_Core.getMainGameInstance` (`GameplayStatics.GetGameInstance`)))
      (set `/Game/AFCore/Blueprints/Game/BP_GameInstance_Main.Chapter Number` 2 _gameinstance))
    (:`then_1`
      (bind _returnvalue (`GameplayStatics.GetActorOfClass` "/Game/Chapters/Chapter2/Blueprint/BP_C2_CSM.BP_C2_CSM_C"))
      (set `self.BP_C2_CSM` _returnvalue)
      (`KismetSystemLibrary.Delay` 0.2)
      (`/Game/Chapters/Chapter2/Blueprint/BP_C2_CSM.Enable Pointer` (`self.BP_C2_CSM`)))
    (:`then_2`
      (bind _returnvalue_2 (`GameplayStatics.GetActorOfClass` "/Game/Chapters/Chapter2/Blueprint/BP_C2RTGCrane.BP_C2RTGCrane_C"))
      (set `self.BP_C2RTGCrane` _returnvalue_2)
      (bind _returnvalue_3 (`GameplayStatics.GetActorOfClass` "/Game/Azureal_Template/VXTemplate/0-Map/Setting/BP_Pawn_VR_VX.BP_Pawn_VR_VX_C"))
      (set `self.BP_Pawn_VR_VX` _returnvalue_3)
      (bind _returnvalue_4 (`GameplayStatics.GetActorOfClass` "/Game/Chapters/Chapter2/Blueprint/BP_ClimbLadder/BP_LeftHook.BP_LeftHook_C"))
      (set `self.BP_LeftHook` _returnvalue_4)
      (bind _returnvalue_5 (`GameplayStatics.GetActorOfClass` "/Game/Chapters/Chapter2/Blueprint/BP_ClimbLadder/BP_RightHook.BP_RightHook_C"))
      (set `self.BP_RightHook` _returnvalue_5)
      (bind _returnvalue_6 (`GameplayStatics.GetActorOfClass` "/Game/Chapters/Chapter2/Blueprint/BP_ClimbLadder/BP_GrabPole.BP_GrabPole_C"))
      (set `self.BP_GrabPole` _returnvalue_6)
      (bind _returnvalue_7 (`GameplayStatics.GetActorOfClass` "/Game/Chapters/Chapter2/Blueprint/BP_ClimbLadder/BP_GrabPole2.BP_GrabPole2_C"))
      (set `self.BP_GrabPole2` _returnvalue_7)
      (bind _returnvalue_8 (`GameplayStatics.GetActorOfClass` "/Game/Chapters/Chapter2/Blueprint/BP_ClimbLadder/BP_GrabPole3.BP_GrabPole3_C"))
      (set `self.BP_GrabPole3` _returnvalue_8)
      (bind _returnvalue_9 (`GameplayStatics.GetActorOfClass` "/Game/Chapters/Chapter2/Blueprint/BP-Boots_Anim.BP-Boots_Anim_C"))
      (set `self.BP-Boots_Anim` _returnvalue_9))
    (:`then_3`
      (bind _foundwidgets (`WidgetBlueprintLibrary.GetAllWidgetsOfClass` "/Game/CSM/Wesport_WBP_StepPage.Wesport_WBP_StepPage_C" false))
      (set `self.Wesport_WBP_StepPage` (`|GetArrayItem` _foundwidgets))
      (`KismetSystemLibrary.Delay` 0.2)
      (`/Game/Azureal_Template/VXTemplate/0-Map/Setting/BP_Pawn_VR_VX.Spawn Harness` (`self.BP_Pawn_VR_VX`)))
    (:`then_4`
      ;[1 1 1] STEP 2
      (`KismetSystemLibrary.Delay` 3.0))
    (:`then_5`
      (bind _returnvalue_10 (`GameplayStatics.GetActorOfClass` "/Game/Chapters/Chapter2/Blueprint/BP_PlayClimbAnimation.BP_PlayClimbAnimation_C"))
      (set `self.BP_PlayClimbAnimation` _returnvalue_10)
      (bind _returnvalue_11 (`GameplayStatics.GetActorOfClass` "/Game/Chapters/Chapter2/Blueprint/BP_ToeBoard.BP_ToeBoard_C"))
      (set `self.BP_ToeBoard` _returnvalue_11)
      (bind _returnvalue_12 (`GameplayStatics.GetActorOfClass` "/Game/Chapters/Chapter2/Blueprint/BP_Scattered_Tools.BP_Scattered_Tools_C"))
      (set `self.BP_Scattered_Tools` _returnvalue_12)
      (bind _returnvalue_13 (`GameplayStatics.GetActorOfClass` "/Game/Chapters/Chapter2/Blueprint/BP_Mud.BP_Mud_C"))
      (set `self.BP_Mud` _returnvalue_13)
      (bind _returnvalue_14 (`GameplayStatics.GetActorOfClass` "/Game/Chapters/Chapter2/Blueprint/BP_Hole.BP_Hole_C"))
      (set `self.BP_Hole` _returnvalue_14)
      (bind _returnvalue_15 (`GameplayStatics.GetActorOfClass` "/Game/Chapters/Chapter2/Blueprint/BP_CraneOperator.BP_CraneOperator_C"))
      (set `self.BP_CraneOperator` _returnvalue_15)
      (bind _returnvalue_16 (`GameplayStatics.GetActorOfClass` "/Game/Chapters/Chapter2/Blueprint/BP_2-3-1.BP_2-3-1_C"))
      (set `self.BP_2-3-1` _returnvalue_16)
      (bind _returnvalue_17 (`GameplayStatics.GetActorOfClass` "/Game/Chapters/Chapter2/Blueprint/BP_ClimbLadder/BP_Hook_AttachPoint_2.BP_Hook_AttachPoint_2_C"))
      (set `self.BP_Hook_AttachPoint_2` _returnvalue_17)
      (bind _returnvalue_18 (`GameplayStatics.GetActorOfClass` "/Game/Chapters/Chapter2/Blueprint/BP_ClimbLadder/BP_Hook_AttachPoint_3.BP_Hook_AttachPoint_3_C"))
      (set `self.BP_Hook_AttachPoint_3` _returnvalue_18))))

(event `StepSequencerInterface.RunStepsOrder`
  (bind _result (`/Engine/EditorBlueprintResources/StandardMacros.IncrementInt` (`self.Steps Interger`))
    (:`  `
      (switch `int` _result
        (:`1`
          (bind _returnvalue (`GameplayStatics.SpawnSound2D` "/Game/Chapters/Steps_Num/1.1" 1.0 1.0 0.0 null))
          (`KismetSystemLibrary.Delay` (`SoundBase.Duration` (`AudioComponent.Sound` _returnvalue)))
          (bind _returnvalue_2 (`GameplayStatics.SpawnSound2D` "/Game/Chapters/Chapter2/Audio/Wes_C2/Step_Intro/C2_Step1.C2_Step1" 1.0 1.0 0.0 null))
          (`KismetSystemLibrary.Delay` (`SoundBase.Duration` (`AudioComponent.Sound` _returnvalue_2)))
          (`self.Step 1`))
        (:`2`
          (bind _returnvalue_3 (`GameplayStatics.SpawnSound2D` "/Game/Chapters/Steps_Num/2.2" 1.0 1.0 0.0 null))
          (`KismetSystemLibrary.Delay` (`SoundBase.Duration` (`AudioComponent.Sound` _returnvalue_3)))
          (bind _returnvalue_4 (`GameplayStatics.SpawnSound2D` "/Game/Chapters/Chapter2/Audio/Wes_C2/Step_Intro/C2_Step2.C2_Step2" 1.0 1.0 0.0 null))
          (`KismetSystemLibrary.Delay` (`SoundBase.Duration` (`AudioComponent.Sound` _returnvalue_4)))
          (`self.Step 2`))
        (:`3`
          (bind _returnvalue_5 (`GameplayStatics.SpawnSound2D` "/Game/Chapters/Steps_Num/3.3" 1.0 1.0 0.0 null))
          (`KismetSystemLibrary.Delay` (`SoundBase.Duration` (`AudioComponent.Sound` _returnvalue_5)))
          (bind _returnvalue_6 (`GameplayStatics.SpawnSound2D` "/Game/Chapters/Chapter2/Audio/Wes_C2/Step_Intro/C2_Step3.C2_Step3" 1.0 1.0 0.0 null))
          (`KismetSystemLibrary.Delay` (`SoundBase.Duration` (`AudioComponent.Sound` _returnvalue_6)))
          (`self.Step 3`))))))

(event `Step 1`
  ;[1 1 1] STEP 1
  (`/Game/Chapters/Chapter2/Blueprint/BP_C2_CSM.Disable Pointer` (`self.BP_C2_CSM`))
  (`/Game/Chapters/Chapter2/Blueprint/BP_C2RTGCrane.Set 1-1-1 Explain Visible` (`self.BP_C2RTGCrane`))
  (`ManualVRPluginBPLibrary.Start`))

(event `Sub 1-1-1`
  ;[1 1 1] SUB 1
  (`/Game/Chapters/Chapter2/Blueprint/BP_C2RTGCrane.Set 1-1-1 Explain Hidden` (`self.BP_C2RTGCrane`))
  ;[1 0.04231 0] Instructions
  (`TrainingStepPage.AdvanceProgress` (`self.Wesport_WBP_StepPage`))
  ;[0.01405 0 1] ManualVR
  (`ManualVRPluginBPLibrary.Update` "2" "1" "1" 1)
  ;[1 1 1] Pointers
  (`/Game/Chapters/Chapter2/Blueprint/BP_C2_CSM.Enable Pointer` (`self.BP_C2_CSM`))
  (`GameplayStatics.SpawnSound2D` "/Game/Chapters/Steps_Completed/1Comp.1Comp" 1.0 1.0 0.0 null))

(event `Sub 2-1-1`
  ;[1 1 1] SUB 2
  (`/Game/Chapters/Chapter2/Blueprint/BP_C2RTGCrane.Set 2-1-1 Explain Hidden` (`self.BP_C2RTGCrane`))
  (`KismetSystemLibrary.Delay` 0.5)
  (`/Game/Chapters/Chapter2/Blueprint/BP_CraneOperator.Set 2-2-1 Explain Visible` (`self.BP_CraneOperator`))
  (`/Game/Chapters/Chapter2/Blueprint/BP_CraneOperator.Spawn Operator` (`self.BP_CraneOperator`))
  (`/Game/Chapters/Chapter2/Blueprint/BP_PlayClimbAnimation.Play Animation Climb` (`self.BP_PlayClimbAnimation`))
  (`KismetSystemLibrary.Delay` 0.1)
  (`/Game/Chapters/Chapter2/Blueprint/BP_PlayClimbAnimation.Pause Animation Climb` (`self.BP_PlayClimbAnimation`))
  (`/Game/Chapters/Chapter2/Blueprint/BP-Boots_Anim.Teleport Beside Ladder` (`self.BP-Boots_Anim`))
  (`/Game/Azureal_Template/VXTemplate/0-Map/Setting/BP_Pawn_VR_VX.Disable Player Movement` (`self.BP_Pawn_VR_VX`))
  ;[1 0.04231 0] Instructions
  (`TrainingStepPage.AdvanceProgress` (`self.Wesport_WBP_StepPage`))
  ;[0.01405 0 1] ManualVR
  (`ManualVRPluginBPLibrary.Update` "2" "2" "1" 1))

(event `Step 2`
  ;[1 1 1] STEP 2
  (`/Game/Chapters/Chapter2/Blueprint/BP_C2RTGCrane.Set 2-1-1 Explain Visible` (`self.BP_C2RTGCrane`)))

(event `Sub 2-2-1`
  ;[1 1 1] SUB 2
  (`/Game/Chapters/Chapter2/Blueprint/BP_CraneOperator.Set 2-2-1 Explain Hidden` (`self.BP_CraneOperator`))
  (`KismetSystemLibrary.Delay` 0.5)
  (`/Game/Chapters/Chapter2/Blueprint/BP_CraneOperator.Set 2-2-2 Explain Visible` (`self.BP_CraneOperator`)))

(event `Sub 2-2-2`
  ;[1 1 1] SUB 2
  (`/Game/Chapters/Chapter2/Blueprint/BP_CraneOperator.Set 2-2-2 Explain Hidden` (`self.BP_CraneOperator`))
  (`KismetSystemLibrary.Delay` 0.5)
  (`/Game/Chapters/Chapter2/Blueprint/BP_CraneOperator.Set 2-2-3 Explain Visible` (`self.BP_CraneOperator`))
  (`/Game/Chapters/Chapter2/Blueprint/BP_PlayClimbAnimation.Play Animation Climb` (`self.BP_PlayClimbAnimation`))
  (`KismetSystemLibrary.Delay` 3.0)
  (`/Game/Chapters/Chapter2/Blueprint/BP_PlayClimbAnimation.Pause Animation Climb` (`self.BP_PlayClimbAnimation`)))

(event `Sub 2-2-3`
  ;[1 1 1] SUB 2
  (`/Game/Chapters/Chapter2/Blueprint/BP_CraneOperator.Set 2-2-3 Explain Hidden` (`self.BP_CraneOperator`))
  (`KismetSystemLibrary.Delay` 0.5)
  (`/Game/Chapters/Chapter2/Blueprint/BP_CraneOperator.Set 2-2-4 Explain Visible` (`self.BP_CraneOperator`))
  (`/Game/Chapters/Chapter2/Blueprint/BP_PlayClimbAnimation.Play Animation Climb` (`self.BP_PlayClimbAnimation`))
  (`KismetSystemLibrary.Delay` 4.0)
  (`/Game/Chapters/Chapter2/Blueprint/BP_PlayClimbAnimation.Pause Animation Climb` (`self.BP_PlayClimbAnimation`)))

(event `Sub 2-2-4`
  ;[1 1 1] SUB 2
  (`/Game/Chapters/Chapter2/Blueprint/BP_CraneOperator.Set 2-2-4 Explain Hidden` (`self.BP_CraneOperator`))
  (`KismetSystemLibrary.Delay` 0.5)
  (`/Game/Chapters/Chapter2/Blueprint/BP_CraneOperator.Set 2-2-5 Explain Visible` (`self.BP_CraneOperator`))
  (`/Game/Chapters/Chapter2/Blueprint/BP_PlayClimbAnimation.Play Animation Climb` (`self.BP_PlayClimbAnimation`))
  (`KismetSystemLibrary.Delay` 2.0)
  (`/Game/Chapters/Chapter2/Blueprint/BP_PlayClimbAnimation.Pause Animation Climb` (`self.BP_PlayClimbAnimation`)))

(event `Sub 2-2-5`
  ;[1 1 1] SUB 2
  (`/Game/Chapters/Chapter2/Blueprint/BP_CraneOperator.Set 2-2-5 Explain Hidden` (`self.BP_CraneOperator`))
  (`KismetSystemLibrary.Delay` 0.5)
  (`/Game/Chapters/Chapter2/Blueprint/BP_CraneOperator.Set 2-2-6 Explain Visible` (`self.BP_CraneOperator`))
  (`/Game/Chapters/Chapter2/Blueprint/BP_PlayClimbAnimation.Play Animation Climb` (`self.BP_PlayClimbAnimation`))
  (`KismetSystemLibrary.Delay` 15.0)
  (`/Game/Chapters/Chapter2/Blueprint/BP_PlayClimbAnimation.Pause Animation Climb` (`self.BP_PlayClimbAnimation`)))

(event `Sub 2-2-6`
  ;[1 1 1] SUB 2
  (`/Game/Chapters/Chapter2/Blueprint/BP_CraneOperator.Set 2-2-6 Explain Hidden` (`self.BP_CraneOperator`))
  (`KismetSystemLibrary.Delay` 0.5)
  (`/Game/Chapters/Chapter2/Blueprint/BP_CraneOperator.Set 2-2-7 Explain Visible` (`self.BP_CraneOperator`)))

(event `Sub 2-2-7-1`
  ;[1 1 1] SUB 2
  (`/Game/Chapters/Chapter2/Blueprint/BP_CraneOperator.Set 2-2-7 Explain Hidden` (`self.BP_CraneOperator`))
  (`/Game/Chapters/Chapter2/Blueprint/BP_ClimbLadder/BP_LeftHook.Spawn Hook Left` (`self.BP_LeftHook`))
  (`/Game/Chapters/Chapter2/Blueprint/BP_ClimbLadder/BP_RightHook.Spawn Hook Right` (`self.BP_RightHook`))
  (`/Game/Chapters/Chapter2/Blueprint/BP-Boots_Anim.Spawn Boots` (`self.BP-Boots_Anim`))
  (`/Game/Chapters/Chapter2/Blueprint/BP_CraneOperator.Hide  Operator` (`self.BP_CraneOperator`))
  (`self.Sub 2-2-7-2`)
  ;[1 0.04231 0] Instructions
  (`TrainingStepPage.AdvanceProgress` (`self.Wesport_WBP_StepPage`))
  ;[0.01405 0 1] ManualVR
  (`ManualVRPluginBPLibrary.Update` "2" "2" "2" 1))

(event `Sub 2-2-7-2`
  ;[1 1 1] SUB 2
  (`/Game/Chapters/Chapter2/Blueprint/BP_2-3-1.Enable Label 2-3-1` (`self.BP_2-3-1`))
  (`/Game/Azureal_Template/VXTemplate/0-Map/Setting/BP_Pawn_VR_VX.Disable Player Movement` (`self.BP_Pawn_VR_VX`))
  (`/Game/Chapters/Chapter2/Blueprint/BP_ClimbLadder/BP_LeftHook.Enable Grab Attach` (`self.BP_LeftHook`))
  (`/Game/Chapters/Chapter2/Blueprint/BP_ClimbLadder/BP_LeftHook.Allow 2-3-1` (`self.BP_LeftHook`))
  (`/Engine/EditorBlueprintResources/StandardMacros.DoOnce` false
    (:`Completed`
      ;[1 0.04231 0] Instructions
      (`/Game/Chapters/Chapter2/Blueprint/BP-Boots_Anim.Teleport To Ladder` (`self.BP-Boots_Anim`)))))

(event `Sub 2-3-1`
  ;[1 1 1] SUB 2
  (`/Game/Chapters/Chapter2/Blueprint/BP_ClimbLadder/BP_LeftHook.Disable Grab Attach` (`self.BP_LeftHook`))
  (`/Game/Chapters/Chapter2/Blueprint/BP_ClimbLadder/BP_LeftHook.Disable 2-3-1` (`self.BP_LeftHook`))
  (`/Game/Chapters/Chapter2/Blueprint/BP_ClimbLadder/BP_GrabPole.Enable Latch Pole1` (`self.BP_GrabPole`))
  (`/Game/Chapters/Chapter2/Blueprint/BP_ClimbLadder/BP_GrabPole.Enable Tag 2-3-2` (`self.BP_GrabPole`)))

(event `Sub 2-3-2`
  ;[1 1 1] SUB 2
  (`/Game/Chapters/Chapter2/Blueprint/BP_ClimbLadder/BP_GrabPole.Disable Latch Pole 1` (`self.BP_GrabPole`))
  (`/Game/Chapters/Chapter2/Blueprint/BP_ClimbLadder/BP_GrabPole.Disable Tag 2-3-2` (`self.BP_GrabPole`))
  (`/Game/Azureal_Template/VXTemplate/0-Map/Setting/BP_Pawn_VR_VX.First MovePlayerUp` (`self.BP_Pawn_VR_VX`))
  (`/Game/Chapters/Chapter2/Blueprint/BP_ClimbLadder/BP_RightHook.Enable Grab Attach` (`self.BP_RightHook`))
  (`/Game/Chapters/Chapter2/Blueprint/BP-Boots_Anim.Left Leg Up` (`self.BP-Boots_Anim`))
  (`/Game/Chapters/Chapter2/Blueprint/BP-Boots_Anim.Play Left 1 Up` (`self.BP-Boots_Anim`)))

(event `Sub 2-3-3`
  ;[1 1 1] SUB 2
  (`/Game/Chapters/Chapter2/Blueprint/BP_ClimbLadder/BP_RightHook.Disable Grab Attach` (`self.BP_RightHook`))
  (`/Game/Chapters/Chapter2/Blueprint/BP_ClimbLadder/BP_GrabPole2.Enable Latch Pole 2` (`self.BP_GrabPole2`))
  (`/Game/Chapters/Chapter2/Blueprint/BP_ClimbLadder/BP_GrabPole2.Enable Tag 2-3-4` (`self.BP_GrabPole2`)))

(event `Sub 2-3-4`
  ;[1 1 1] SUB 2
  (`/Game/Chapters/Chapter2/Blueprint/BP_ClimbLadder/BP_GrabPole2.Disable Latch Pole 2` (`self.BP_GrabPole2`))
  (`/Game/Chapters/Chapter2/Blueprint/BP_ClimbLadder/BP_GrabPole2.Disable Tag 2-3-4` (`self.BP_GrabPole2`))
  (`/Game/Azureal_Template/VXTemplate/0-Map/Setting/BP_Pawn_VR_VX.First MovePlayerUp` (`self.BP_Pawn_VR_VX`))
  (`/Game/Chapters/Chapter2/Blueprint/BP-Boots_Anim.Pause Left 1 Up` (`self.BP-Boots_Anim`))
  (`/Game/Chapters/Chapter2/Blueprint/BP-Boots_Anim.Right Leg Up` (`self.BP-Boots_Anim`))
  (`/Game/Chapters/Chapter2/Blueprint/BP-Boots_Anim.Play Right 1 Up` (`self.BP-Boots_Anim`))
  (`KismetSystemLibrary.Delay` 0.2)
  (`/Game/Chapters/Chapter2/Blueprint/BP_ClimbLadder/BP_LeftHook.Enable Grab Attach 2` (`self.BP_LeftHook`))
  (`/Game/Chapters/Chapter2/Blueprint/BP_ClimbLadder/BP_LeftHook.Allow 2-3-5` (`self.BP_LeftHook`)))

(event `Sub 2-3-5`
  ;[1 1 1] SUB 2
  (`/Game/Chapters/Chapter2/Blueprint/BP_ClimbLadder/BP_LeftHook.Disable Grab Attach 2` (`self.BP_LeftHook`))
  (`/Game/Chapters/Chapter2/Blueprint/BP_ClimbLadder/BP_LeftHook.Disable 2-3-5` (`self.BP_LeftHook`))
  (`/Game/Chapters/Chapter2/Blueprint/BP_ClimbLadder/BP_GrabPole3.Enable Latch Pole 3` (`self.BP_GrabPole3`)))

(event `Sub 2-3-6`
  ;[1 1 1] SUB 2
  (`/Game/Chapters/Chapter2/Blueprint/BP-Boots_Anim.Pause Right 1 Up` (`self.BP-Boots_Anim`))
  (`/Game/Chapters/Chapter2/Blueprint/BP_ClimbLadder/BP_GrabPole3.Disable Latch Pole 3` (`self.BP_GrabPole3`))
  (`/Game/Azureal_Template/VXTemplate/0-Map/Setting/BP_Pawn_VR_VX.First MovePlayerUp` (`self.BP_Pawn_VR_VX`))
  (`/Game/Chapters/Chapter2/Blueprint/BP-Boots_Anim.Left Leg Up 2` (`self.BP-Boots_Anim`))
  (`/Game/Chapters/Chapter2/Blueprint/BP-Boots_Anim.Play Left 2 Up` (`self.BP-Boots_Anim`))
  (`KismetSystemLibrary.Delay` 2.0)
  (`/Game/Chapters/Chapter2/Blueprint/BP-Boots_Anim.Teleport To Stair` (`self.BP-Boots_Anim`))
  (`/Game/Azureal_Template/VXTemplate/0-Map/Setting/BP_Pawn_VR_VX.Ending Climbing` (`self.BP_Pawn_VR_VX`))
  (`/Game/Azureal_Template/VXTemplate/0-Map/Setting/BP_Pawn_VR_VX.Enable Player Movement` (`self.BP_Pawn_VR_VX`))
  (`/Game/Chapters/Chapter2/Blueprint/BP_C2_CSM.Move Menu Upstairs` (`self.BP_C2_CSM`))
  (`/Game/Chapters/Chapter2/Blueprint/BP_2-3-1.Disable Label 2-3-1` (`self.BP_2-3-1`))
  (`/Game/Chapters/Chapter2/Blueprint/BP-Boots_Anim.Hide Boots` (`self.BP-Boots_Anim`))
  (`/Game/Chapters/Chapter2/Blueprint/BP_2-3-1.Disable Label 2-3-1` (`self.BP_2-3-1`))
  ;[1 0.04231 0] Instructions
  (`TrainingStepPage.AdvanceProgress` (`self.Wesport_WBP_StepPage`))
  ;[0.01405 0 1] ManualVR
  (`ManualVRPluginBPLibrary.Update` "2" "2" "3" 1)
  ;[1 1 1] Pointers
  (`/Game/Chapters/Chapter2/Blueprint/BP_C2_CSM.Enable Pointer` (`self.BP_C2_CSM`))
  (`GameplayStatics.SpawnSound2D` "/Game/Chapters/Steps_Completed/2Comp.2Comp" 1.0 1.0 0.0 null))

(event `Reset Everything`
  ;[1 1 1] SUB 2
  (`/Game/Chapters/Chapter2/Blueprint/BP_ClimbLadder/BP_GrabPole.Reset Pole 1` (`self.BP_GrabPole`))
  (`/Game/Chapters/Chapter2/Blueprint/BP_ClimbLadder/BP_GrabPole2.Reset Pole 2` (`self.BP_GrabPole2`))
  (`/Game/Chapters/Chapter2/Blueprint/BP_ClimbLadder/BP_GrabPole2.Disable Latch Pole 2` (`self.BP_GrabPole2`))
  (`/Game/Chapters/Chapter2/Blueprint/BP_ClimbLadder/BP_LeftHook.Disable 2-3-1` (`self.BP_LeftHook`))
  (`/Game/Chapters/Chapter2/Blueprint/BP_ClimbLadder/BP_LeftHook.Disable 2-3-5` (`self.BP_LeftHook`))
  (`/Game/Chapters/Chapter2/Blueprint/BP-Boots_Anim.Reset Anim L` (`self.BP-Boots_Anim`))
  (`/Game/Chapters/Chapter2/Blueprint/BP-Boots_Anim.Reset Anim R` (`self.BP-Boots_Anim`))
  (`/Game/Chapters/Chapter2/Blueprint/BP_ClimbLadder/BP_GrabPole3.Disable Latch Pole 3` (`self.BP_GrabPole3`))
  (`/Game/Chapters/Chapter2/Blueprint/BP_ClimbLadder/BP_LeftHook.Reset Hook Left` (`self.BP_LeftHook`))
  (`/Game/Chapters/Chapter2/Blueprint/BP_ClimbLadder/BP_RightHook.Reset Hook Right` (`self.BP_RightHook`))
  (`/Game/Chapters/Chapter2/Blueprint/BP_ClimbLadder/BP_GrabPole2.Disable Tag 2-3-4` (`self.BP_GrabPole2`)))

(event `Sub 3-1-1`
  ;[1 1 1] SUB 3
  (`/Game/Chapters/Chapter2/Blueprint/BP_C2RTGCrane.Set 3-1-1 Explain Hidden` (`self.BP_C2RTGCrane`))
  (`KismetSystemLibrary.Delay` 0.5)
  (`/Game/Chapters/Chapter2/Blueprint/BP_C2RTGCrane.Set 3-1-2 Explain Visible` (`self.BP_C2RTGCrane`)))

(event `Step 3`
  ;[1 1 1] STEP 3
  (`KismetSystemLibrary.Delay` 0.2)
  (`/Game/Chapters/Chapter2/Blueprint/BP_C2RTGCrane.Set 3-1-1 Explain Visible` (`self.BP_C2RTGCrane`)))

(event `Sub 3-1-2`
  ;[1 1 1] SUB 3
  (`/Game/Chapters/Chapter2/Blueprint/BP_C2RTGCrane.Set 3-1-2 Explain Hidden` (`self.BP_C2RTGCrane`))
  (`KismetSystemLibrary.Delay` 0.5)
  (`/Game/Chapters/Chapter2/Blueprint/BP_C2RTGCrane.Set 3-2-1 Explain Visible` (`self.BP_C2RTGCrane`))
  ;[1 0.04231 0] Instructions
  (`TrainingStepPage.AdvanceProgress` (`self.Wesport_WBP_StepPage`))
  ;[0.01405 0 1] ManualVR
  (`ManualVRPluginBPLibrary.Update` "2" "3" "1" 1))

(event `Sub 3-2-1-1`
  ;[1 1 1] SUB 3
  (`/Game/Chapters/Chapter2/Blueprint/BP_C2RTGCrane.Set 3-2-1 Explain Hidden` (`self.BP_C2RTGCrane`))
  (`/Game/Chapters/Chapter2/Blueprint/BP_C2RTGCrane.Enable Gaze` (`self.BP_C2RTGCrane`)))

(event `Sub 3-2-1-2`
  ;[1 1 1] SUB 3
  (`/Game/Chapters/Chapter2/Blueprint/BP_C2RTGCrane.Disable Gaze` (`self.BP_C2RTGCrane`))
  (`/Game/Chapters/Chapter2/Blueprint/BP_C2RTGCrane.Set 3-2-2 Explain Visible` (`self.BP_C2RTGCrane`)))

(event `Sub 3-2-2-1`
  ;[1 1 1] SUB 3
  (`/Game/Chapters/Chapter2/Blueprint/BP_C2RTGCrane.Set 3-2-2 Explain Hidden` (`self.BP_C2RTGCrane`))
  (`/Game/Chapters/Chapter2/Blueprint/BP_ToeBoard.Enable Gaze` (`self.BP_ToeBoard`)))

(event `Sub 3-2-2-2`
  ;[1 1 1] SUB 3
  (`/Game/Chapters/Chapter2/Blueprint/BP_ToeBoard.Disable Gaze` (`self.BP_ToeBoard`))
  (`/Game/Chapters/Chapter2/Blueprint/BP_ToeBoard.Set 3-2-3 Explain Visible` (`self.BP_ToeBoard`)))

(event `Sub 3-2-3`
  ;[1 1 1] SUB 3
  (`/Game/Chapters/Chapter2/Blueprint/BP_ToeBoard.Set 3-2-3 Explain Hidden` (`self.BP_ToeBoard`))
  (`KismetSystemLibrary.Delay` 0.5)
  (`/Game/Chapters/Chapter2/Blueprint/BP_C2RTGCrane.Set 3-3-1 Explain Visible` (`self.BP_C2RTGCrane`))
  ;[1 0.04231 0] Instructions
  (`TrainingStepPage.AdvanceProgress` (`self.Wesport_WBP_StepPage`))
  ;[0.01405 0 1] ManualVR
  (`ManualVRPluginBPLibrary.Update` "2" "3" "2" 1))

(event `Sub 3-3-1`
  ;[1 1 1] SUB 3
  (`/Game/Chapters/Chapter2/Blueprint/BP_C2RTGCrane.Set 3-3-1 Explain Hidden` (`self.BP_C2RTGCrane`))
  (`KismetSystemLibrary.Delay` 0.5)
  (`/Game/Chapters/Chapter2/Blueprint/BP_Scattered_Tools.Enable Gaze` (`self.BP_Scattered_Tools`)))

(event `Sub 3-3-2-1`
  ;[1 1 1] SUB 3
  (`/Game/Chapters/Chapter2/Blueprint/BP_Scattered_Tools.Disable Gaze` (`self.BP_Scattered_Tools`))
  (`/Game/Chapters/Chapter2/Blueprint/BP_Scattered_Tools.Set 3-3-2 Explain Visible` (`self.BP_Scattered_Tools`)))

(event `Sub 3-3-2-2`
  ;[1 1 1] SUB 3
  (`/Game/Chapters/Chapter2/Blueprint/BP_Scattered_Tools.Set 3-3-2 Explain Hidden` (`self.BP_Scattered_Tools`))
  (`/Game/Chapters/Chapter2/Blueprint/BP_Scattered_Tools.Hide Tools` (`self.BP_Scattered_Tools`))
  (`/Game/Chapters/Chapter2/Blueprint/BP_Mud.Enable Gaze` (`self.BP_Mud`)))

(event `Sub 3-3-3-1`
  ;[1 1 1] SUB 3
  (`/Game/Chapters/Chapter2/Blueprint/BP_Mud.Disable Gaze` (`self.BP_Mud`))
  (`/Game/Chapters/Chapter2/Blueprint/BP_Mud.Set 3-3-2 Explain Visible` (`self.BP_Mud`)))

(event `Sub 3-3-3-2`
  ;[1 1 1] SUB 3
  (`/Game/Chapters/Chapter2/Blueprint/BP_Mud.Set 3-3-2 Explain Hidden` (`self.BP_Mud`))
  (`/Game/Chapters/Chapter2/Blueprint/BP_Mud.Hide Mud` (`self.BP_Mud`))
  (`/Game/Chapters/Chapter2/Blueprint/BP_Hole.Enable Gaze` (`self.BP_Hole`))
  (`/Game/Chapters/Chapter2/Blueprint/BP_C2RTGCrane.Show Crane Hole` (`self.BP_C2RTGCrane`)))

(event `Sub 3-3-4-1`
  ;[1 1 1] SUB 3
  (`/Game/Chapters/Chapter2/Blueprint/BP_Hole.Disable Gaze` (`self.BP_Hole`))
  (`/Game/Chapters/Chapter2/Blueprint/BP_Hole.Set 3-3-4 Explain Visible` (`self.BP_Hole`)))

(event `Sub 3-3-4-2`
  ;[1 1 1] SUB 3
  (`/Game/Chapters/Chapter2/Blueprint/BP_Hole.Set 3-3-4 Explain Hidden` (`self.BP_Hole`))
  (`/Game/Chapters/Chapter2/Blueprint/BP_Hole.Hide Hole` (`self.BP_Hole`))
  (`/Game/Chapters/Chapter2/Blueprint/BP_C2RTGCrane.Hide Crane Hole` (`self.BP_C2RTGCrane`))
  (`KismetSystemLibrary.Delay` 0.5)
  (`/Game/Chapters/Chapter2/Blueprint/BP_C2RTGCrane.Set 3-3-5 Explain Visible` (`self.BP_C2RTGCrane`)))

(event `Sub 3-3-5`
  ;[1 1 1] SUB 3
  (`/Game/Chapters/Chapter2/Blueprint/BP_C2RTGCrane.Set 3-3-5 Explain Hidden` (`self.BP_C2RTGCrane`))
  (`KismetSystemLibrary.Delay` 0.5)
  (`/Game/Chapters/Chapter2/Blueprint/BP_C2RTGCrane.Set 3-3-6 Explain Visible` (`self.BP_C2RTGCrane`)))

(event `Sub 3-3-6`
  ;[1 1 1] SUB 3
  (`/Game/Chapters/Chapter2/Blueprint/BP_C2RTGCrane.Set 3-3-6 Explain Hidden` (`self.BP_C2RTGCrane`))
  ;[1 0.04231 0] Instructions
  (`TrainingStepPage.AdvanceProgress` (`self.Wesport_WBP_StepPage`))
  ;[0.01405 0 1] ManualVR
  (`ManualVRPluginBPLibrary.Update` "2" "3" "3" 1)
  ;[1 1 1] Pointers
  (`/Game/Chapters/Chapter2/Blueprint/BP_C2_CSM.Enable Pointer` (`self.BP_C2_CSM`))
  (`GameplayStatics.SpawnSound2D` "/Game/Chapters/Steps_Completed/3Comp.3Comp" 1.0 1.0 0.0 null)
  (`ManualVRPluginBPLibrary.End`))

(event `Step 4`
  ;[1 1 1] STEP 4
)

(event `Sub 4-1-1`
  ;[1 1 1] SUB 4
)

(event `Sub 4-1-2`
  ;[1 1 1] SUB 4
)

(event `Sub 4-1-3`
  ;[1 1 1] SUB 4
)

(event `Sub 4-1-4`
  ;[1 1 1] SUB 4
)

(event `Sub 4-1-5`
  ;[1 1 1] SUB 4
)

(event `Sub 4-1-6`
  ;[1 1 1] SUB 4
)

(fn `UserConstructionScript`)