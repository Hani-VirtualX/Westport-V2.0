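; BP_Hole is a Chapter 2 gaze-interactable hole that advances step 3-3-4 of the chapter.
; Events toggle its gaze prompt and explanation label through the VXGaze and VXExplain components, and can hide the cube mesh.
; After a short BeginPlay delay it caches BP_GazeIndicator, whose progress bar resets when gaze is disabled, and GM_C2.
; A completed gaze trigger calls Sub3341 on GM_C2 only once.
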(event `self.ReceiveBeginPlay`
  (`KismetSystemLibrary.Delay` 0.2)
  (bind _returnvalue (`GameplayStatics.GetActorOfClass` "/Game/AFCore/Blueprints/UI/GazeIndicator/BP_GazeIndicator.BP_GazeIndicator_C"))
  (set `self.Gaze` _returnvalue)
  (bind _returnvalue_2 (`GameplayStatics.GetActorOfClass` "/Game/Chapters/Chapter2/Blueprint/GM_C2.GM_C2_C"))
  (set `self.GM_C2` _returnvalue_2))

(event `Enable Gaze`
  ;[1 1 1] Gaze
  (`/Game/Azureal_Template/VX_Gaze/VX_Gaze.Set [ Gaze ]` (`self.VX_Gaze`) (`self.Cube`) (`self.Gaze_Label`) true "NewEnumerator7" "NewEnumerator0" "NewEnumerator1" "NewEnumerator0"))

(event `Disable Gaze`
  ;[1 1 1] Gaze
  (`/Game/Azureal_Template/VX_Gaze/VX_Gaze.Set [ Gaze ]` (`self.VX_Gaze`) (`self.Cube`) (`self.Gaze_Label`) false "NewEnumerator6" "NewEnumerator4" "NewEnumerator4" "NewEnumerator4")
  (`/Game/AFCore/Blueprints/UI/GazeIndicator/BP_GazeIndicator.Reset Progress Bar` (`self.Gaze`)))

(event `Set 3-3-4 Explain Visible`
  ;[1 0.1979 1] Explains
  (`/Game/Azureal_Template/VX_Explain/VX_Explain.Set [ Explain + ]` (`self.VX_Explain`) (`self.Cube`) (`self.3-3-4 Exp`) true "NewEnumerator6" "NewEnumerator7" "NewEnumerator0" "NewEnumerator1" "NewEnumerator0"))

(event `Set 3-3-4 Explain Hidden`
  ;[1 0.1979 1] Explains
  (`/Game/Azureal_Template/VX_Explain/VX_Explain.Set [ Explain + ]` (`self.VX_Explain`) (`self.Cube`) (`self.3-3-4 Exp`) false "NewEnumerator6" "NewEnumerator6" "NewEnumerator4" "NewEnumerator4" "NewEnumerator4"))

(event `self.VX_Gaze.Gaze Triggered`
  ;[1 1 1] Gaze
  (`/Engine/EditorBlueprintResources/StandardMacros.DoOnce` false
    (:`Completed`
      (`/Game/Chapters/Chapter2/Blueprint/GM_C2.Sub 3-3-4-1` (`self.GM_C2`)))))

(event `Hide Hole`
  (`SceneComponent.SetHiddenInGame` (`self.Cube`) true false))

(fn `UserConstructionScript`)