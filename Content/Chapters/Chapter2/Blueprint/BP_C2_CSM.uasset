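; BP_C2_CSM is a Chapter 2 actor that can be moved upstairs as a menu and can switch a VX pointer on or off.
; Shortly after BeginPlay it finds and caches the VX_Pointer_Widget actor, then forwards enable calls with its Widget and disable calls to it.
; MoveMenuUpstairs repositions the actor's root to a stored location and rotation.
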(event `self.ReceiveBeginPlay`
  (`KismetSystemLibrary.Delay` 0.2)
  (bind _returnvalue (`GameplayStatics.GetActorOfClass` "/Game/Azureal_Template/VX_WidgetMasterArrow/VX_Pointer_Widget.VX_Pointer_Widget_C"))
  (set `self.VX Pointer` _returnvalue))

(event `Move Menu Upstairs`
  (`SceneComponent.K2_SetWorldLocationAndRotation` (`self.DefaultSceneRoot`) (`self.New Location`) (`self.New Rotation`) false false))

(event `Enable Pointer`
  (`/Game/Azureal_Template/VX_WidgetMasterArrow/VX_Pointer_Widget.Enable Pointer` (`self.VX Pointer`) (`self.Widget`)))

(event `Disable Pointer`
  (`/Game/Azureal_Template/VX_WidgetMasterArrow/VX_Pointer_Widget.Disable Pointer` (`self.VX Pointer`)))

(fn `UserConstructionScript`)