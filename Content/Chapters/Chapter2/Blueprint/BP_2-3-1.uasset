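; BP_2-3-1 is a Chapter 2 Blueprint for step 2-3-1 that shows and hides a label widget.
; Two custom events, EnableLabel2-3-1 and DisableLabel2-3-1, pass the Label to VXLabel.SetLabel, with Visible set only when enabling.
; It has no active BeginPlay, Tick, overlap or construction logic, and two leftover SetHiddenInGame nodes are never run.
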(event `Enable Label 2-3-1`
  (`/Game/Azureal_Template/VX_Label/VX_Label.Set [ Label ]` (`self.VX_Label`) null (`self.Label`) true "NewEnumerator6" "NewEnumerator4" "NewEnumerator4"))

(event `Disable Label 2-3-1`
  (`/Game/Azureal_Template/VX_Label/VX_Label.Set [ Label ]` (`self.VX_Label`) null (`self.Label`) false "NewEnumerator6" "NewEnumerator4" "NewEnumerator4"))

(fn `UserConstructionScript`)