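; BP_TestRTGCrane is the RTG crane actor for Chapter 2's test, hosting step-by-step explanations and a crane-hole material swap.
; Show/hide events toggle each step's explain component, using basic or "Plus" variants.
; Completion callbacks fire once to call matching Sub functions on GM_TestC2, cached shortly after BeginPlay; Plus variants require StepIndex 2, and Step 3-2-2's callback is empty.
; ShowCraneHole and HideCraneHole swap the crane mesh's first material.
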(event `self.ReceiveBeginPlay`
  (`KismetSystemLibrary.Delay` 0.2)
  (bind _returnvalue (`GameplayStatics.GetActorOfClass` "/Game/Chapters/NEW_C2/BP/GM_TestC2.GM_TestC2_C"))
  (set `self.GM_TestC2` _returnvalue))

(event `Set 1-1-1 Explain Visible`
  (`Azr_Explain.EnableExplain` (`self.Step1_Explain`)))

(event `Set 1-1-1 Explain Hidden`
  (`Azr_Explain.DisableExplain` (`self.Step1_Explain`)))

(event `Set 2-1-1 Explain Visible`
  (`Azr_Explain.EnableExplain` (`self.Step2_Explain`)))

(event `Set 2-1-1 Explain Hidden`
  (`Azr_Explain.DisableExplain` (`self.Step2_Explain`)))

(event `Set 3-1-1 Explain Hidden`
  (`Azr_Explain.DisableExplain` (`self.Step3-1_Explain`)))

(event `Set 3-1-1 Explain Visible`
  (`Azr_Explain.EnableExplainPlus` (`self.Step3-1_Explain`)))

(event `Set 3-2-1 Explain Visible`
  (`Azr_Explain.EnableExplain` (`self.Step3-2-1_Explain`)))

(event `Set 3-2-1 Explain Hidden`
  (`Azr_Explain.DisableExplain` (`self.Step3-2-1_Explain`)))

(event `Set 3-2-2 Explain Visible`
  (`Azr_Explain.EnableExplain` (`self.Step3-2-2_Explain`)))

(event `Set 3-2-2 Explain Hidden`
  (`Azr_Explain.DisableExplain` (`self.Step3-2-2_Explain`)))

(event `Set 3-3-1 Explain Visible`
  (`Azr_Explain.EnableExplain` (`self.Step3-3-1_Explain`)))

(event `Set 3-3-1 Explain Hidden`
  (`Azr_Explain.DisableExplain` (`self.Step3-3-1_Explain`)))

(event `Show Crane Hole`
  (`PrimitiveComponent.SetMaterial` (`self.WP_RTGCrane_Joined`) 0 "/Game/wesport_Stuff/Assets/RTGCrane/Materials/RTG_Bottom_Inst_Hole.RTG_Bottom_Inst_Hole"))

(event `Hide Crane Hole`
  (`PrimitiveComponent.SetMaterial` (`self.WP_RTGCrane_Joined`) 0 "/Game/wesport_Stuff/Assets/RTGCrane/Materials/RTG_Bottom_Inst.RTG_Bottom_Inst"))

(event `Set 3-3-5 Explain Visible`
  (`Azr_Explain.EnableExplainPlus` (`self.Step3-3-5_Explain`)))

(event `Set 3-3-5 Explain Hidden`
  (`Azr_Explain.DisableExplain` (`self.Step3-3-5_Explain`)))

(event `self.Step1_Explain.OnExplainCompleted`
  (`/Engine/EditorBlueprintResources/StandardMacros.DoOnce` false
    (:`Completed`
      (`/Game/Chapters/NEW_C2/BP/GM_TestC2.Sub 1-1-1` (`self.GM_TestC2`)))))

(event `self.Step2_Explain.OnExplainCompleted`
  (`/Engine/EditorBlueprintResources/StandardMacros.DoOnce` false
    (:`Completed`
      (`/Game/Chapters/NEW_C2/BP/GM_TestC2.Sub 2-1-1` (`self.GM_TestC2`)))))

(event `self.Step3-2-1_Explain.OnExplainCompleted`
  (`/Engine/EditorBlueprintResources/StandardMacros.DoOnce` false
    (:`Completed`
      (`/Game/Chapters/NEW_C2/BP/GM_TestC2.Sub 3-2-1-1` (`self.GM_TestC2`)))))

(event `self.Step3-2-2_Explain.OnExplainCompleted`
  (`/Engine/EditorBlueprintResources/StandardMacros.DoOnce` false))

(event `self.Step3-3-1_Explain.OnExplainCompleted`
  (`/Engine/EditorBlueprintResources/StandardMacros.DoOnce` false
    (:`Completed`
      (`/Game/Chapters/NEW_C2/BP/GM_TestC2.Sub 3-3-1` (`self.GM_TestC2`)))))

(event `self.Step3-1_Explain.OnExplainPlusCompleted`
  (params (StepIndex :type Integer))
  (switch `int` StepIndex
    (:`2`
      (`/Engine/EditorBlueprintResources/StandardMacros.DoOnce` false
        (:`Completed`
          (`/Game/Chapters/NEW_C2/BP/GM_TestC2.Sub 3-1-1` (`self.GM_TestC2`)))))))

(event `self.Step3-3-5_Explain.OnExplainPlusCompleted`
  (params (StepIndex :type Integer))
  (switch `int` StepIndex
    (:`2`
      (`/Engine/EditorBlueprintResources/StandardMacros.DoOnce` false
        (:`Completed`
          (`/Game/Chapters/NEW_C2/BP/GM_TestC2.Sub 3-3-5` (`self.GM_TestC2`)))))))

(fn `UserConstructionScript`)